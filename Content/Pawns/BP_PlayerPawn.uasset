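; BP_PlayerPawn is a player pawn with two spring-arm cameras, input-driven camera swap and zoom, and a level reset.
; A FlipFlop toggles Camera on swap input, though both branches activate CameraLeft.
; Holding ZoomIn plays a timeline per spring arm, setting arm length and zeroing socket offset, reversing on release, without checking which camera is active.
; ResetLevel opens the Sandbox level by name.
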(event EventBeginPlay
  (|CallParentFunction))

(event Collision|EventActorBeginOverlap
  (params (OtherActor :type Actor%20Object%20Reference))
  (|CallParentFunction OtherActor) ; This node is disabled and will not be called.\nDrag off pins to build functionality.
)

(event EventTick
  (params (DeltaSeconds :type Float%20%28single-precision%29))
  (|CallParentFunction DeltaSeconds) ; This node is disabled and will not be called.\nDrag off pins to build functionality.
)

(event Input|ActionEvents|InputActionCameraSwap
  (params (Key :type Key%20Structure :default "None"))
  ;[1 1 1] Camera swap (V)
  (:Pressed
    (Utilities|FlowControl|FlipFlop
      (:A
        (Components|Activation|SetActive (Variables|Default|GetCamera) false false)
        (Components|Activation|SetActive (Variables|Default|GetCameraLeft) true false))
      (:B
        (Components|Activation|SetActive (Variables|Default|GetCamera) true false)
        (Components|Activation|SetActive (Variables|Default|GetCameraLeft) true false)))))

(event Input|ActionEvents|InputActionResetLevel
  (params (Key :type Key%20Structure :default "None"))
  ;[1 1 1] Reset Level (Y)
  (:Pressed
    (Game|OpenLevel(byName) "Sandbox")))

(event Input|ActionEvents|InputActionZoomIn
  (params (Key :type Key%20Structure :default "None"))
  (bind _springarmleft (Variables|Default|GetSpringArmLeft))
  ;[1 1 1] ZoomIn and Out (RightMouseButton
  ;;[1 1 1] ZoomIn when second Camera Active
  (:Pressed
    (bind _arm_length (Timeline|Timeline_0 Play)
      (:Update
        (Variables|/Script/Engine.SpringArmComponent|SetTargetArmLength _springarmleft _arm_length)
        (Variables|/Script/Engine.SpringArmComponent|SetSocketOffset _springarmleft "0, 0, 0"))))
  (:Released
    (Timeline|Timeline_0 Reverse)))

(event Input|ActionEvents|InputActionZoomIn
  (params (Key :type Key%20Structure :default "None"))
  (bind _springarm (Variables|Default|GetSpringArm))
  ;[1 1 1] ZoomIn and Out (RightMouseButton
  ;;[1 1 1] ZoomIn when Basic Camera Active
  (:Pressed
    (bind _arm_length (Timeline|Zoom Play)
      (:Update
        (Variables|/Script/Engine.SpringArmComponent|SetTargetArmLength _springarm _arm_length)
        (Variables|/Script/Engine.SpringArmComponent|SetSocketOffset _springarm "0, 0, 0"))))
  (:Released
    (Timeline|Zoom Reverse)))

(fn ConstructionScript
  (|CallParentFunction))