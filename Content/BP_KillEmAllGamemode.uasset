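; BP_KillEmAllGamemode is a game mode Blueprint that keeps the elapsed game time, noted as working with a widget.
; While IsGameRunning is true, Tick adds DeltaSeconds to Miliseconds, which actually holds fractional seconds, and carries overflow into Seconds and then Minutes.
; It only maintains these counters; BeginPlay and the construction script are empty, and nothing here sets the running flag or updates the widget.
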(event EventBeginPlay)

(event EventTick
  (params (DeltaSeconds :type Float%20%28single-precision%29))
  ;[1 0.8845 0.8746] Timer (working with widget)
  (if (Variables|Default|GetIsGameRunning)
    (Variables|Default|SetMiliseconds (+ DeltaSeconds (Variables|Default|GetMiliseconds)))
    (if (> (Variables|Default|GetMiliseconds) 1)
      (Variables|Default|SetSeconds (+ 1 (Variables|Default|GetSeconds)))
      (Variables|Default|SetMiliseconds (- (Variables|Default|GetMiliseconds) 1.0))
      (if (>= (Variables|Default|GetSeconds) 60)
        (Variables|Default|SetMinutes (+ (Variables|Default|GetMinutes) 1))
        (Variables|Default|SetSeconds (- (Variables|Default|GetSeconds) 60))))))

(fn ConstructionScript)